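; Treasure chest interactable Blueprint, where Interact calls the parent implementation and prints a debug string.
; Two disconnected graph fragments never run: a key-card gameplay tag check against the action component, and a FlipFlop timeline that pitches the lid open or closed and activates particles once finished.
; Any working chest behavior therefore comes from the parent class, outside this graph.
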(event `SGameplayInterface.Interact`
  (params (InstigatorPawn :type "Pawn Object Reference"))
  (`parent.Interact` InstigatorPawn)
  (`KismetSystemLibrary.PrintString` "TreasureChest(BP)" true true (struct :`A` 1.0) 10.0))

(fn `UserConstructionScript`)