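; Base interactable fire light actor that the player can toggle on and off.
; Interact flips ActivateFire based on FireActivated, then calls UpdateFlames to switch three particle systems and a light together and record the new state.
; OnActorLoaded also calls UpdateFlames to reapply the state on load.
; Both state variables have empty RepNotify functions, and GetInteractText returns a variable as the prompt.
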(event `UpdateFlames`
  (bind _particlesystemcomponent02 (`self.ParticleSystemComponent02`))
  (bind _lightcomponent0 (`self.LightComponent0`))
  (if (`self.ActivateFire`)
    (`ActorComponent.Activate` _particlesystemcomponent02 false)
    (`ActorComponent.Activate` (`self.ParticleSystemComponent01`) false)
    (`ActorComponent.Activate` (`self.ParticleSystemComponent0`) false)
    (`SceneComponent.SetVisibility` _lightcomponent0 true false)
    (set `self.FireActivated` true)
    (else
      (`ActorComponent.Deactivate` _particlesystemcomponent02)
      (`ActorComponent.Deactivate` (`self.ParticleSystemComponent01`))
      (`ActorComponent.Deactivate` (`self.ParticleSystemComponent0`))
      (`SceneComponent.SetVisibility` _lightcomponent0 false false)
      (set `self.FireActivated` false))))

(event `SGameplayInterface.Interact`
  (params (InstigatorPawn :type "Pawn Object Reference"))
  (if (`self.FireActivated`)
    (set `self.ActivateFire` false)
    (else
      (set `self.ActivateFire` true)))
  (`self.UpdateFlames`))

(event `SGameplayInterface.OnActorLoaded`
  (`self.UpdateFlames`))

(fn `GetInteractText`
  (params (InsitgatorPawn :type "Pawn Object Reference"))
  (returns (ReturnValue :type Text))
  (return (`self.NewVar_0`)))

(fn `OnRep_ActivateFire`)

(fn `OnRep_FireActivated`)

(fn `UserConstructionScript`)