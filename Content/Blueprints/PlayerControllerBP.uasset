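; Player controller Blueprint that sets up the main HUD and opens a quest journal.
; On BeginPlay it adds Main_HUD to the viewport and sets game-only input.
; NumPad 3 creates and shows a new BP_QuestJournal fed by TeamActor's shared Narrative component.
; The chain that finds TeamActor from BP_CoOp and creates the default Narrative UI is disconnected, so nothing here assigns TeamActor at runtime.
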(event `self.ReceiveBeginPlay`
  (bind _returnvalue (`|CreateWidget` "/Game/Blueprints/UMG/Main_HUD.Main_HUD_C" (`GameplayStatics.GetPlayerController` 0)))
  (`UserWidget.AddToViewport` _returnvalue 0)
  (`WidgetBlueprintLibrary.SetInputMode_GameOnly` self))

(event `Key|NumPadThree`
  (params (Key :type "Key Structure"))
  (:`Pressed`
    (bind _returnvalue (`|CreateWidget` "/Narrative/NarrativeUI/Widgets/BP_QuestJournal.BP_QuestJournal_C" null (`/Game/Blueprints/Narrative/BP_Co-Op.SharedNarrativeComponent` (`self.TeamActor`))))
    (`UserWidget.AddToViewport` _returnvalue 0)))

(fn `UserConstructionScript`)