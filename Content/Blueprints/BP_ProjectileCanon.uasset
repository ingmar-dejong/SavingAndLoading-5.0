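; BP_ProjectileCanon is a cannon actor that periodically fires BP_MagicProjectile actors.
; A looping two-second timer started on BeginPlay spawns each projectile at the actor's own location and rotation.
; Each tick rotates only the Arrow component to face player pawn 0, so the spawn rotation does not use that aim.
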(event `self.ReceiveBeginPlay`
  (`KismetSystemLibrary.K2_SetTimerDelegate` (delegate `TimeElapsed`) 2.0 true))

(event `TimeElapsed`
  (`|SpawnActorFromClass` "/Game/Blueprints/BP_MagicProjectile.BP_MagicProjectile_C" (`KismetMathLibrary.MakeTransform` (`self.K2_GetActorLocation`) (`self.K2_GetActorRotation`)) "Undefined" "OverrideRootScale" null null))

(event `self.ReceiveTick`
  (params (DeltaSeconds :type "Float (single-precision)"))
  (`SceneComponent.K2_SetWorldRotation` (`self.Arrow`) (`KismetMathLibrary.FindLookAtRotation` (`self.K2_GetActorLocation`) (`self.K2_GetActorLocation` (`GameplayStatics.GetPlayerPawn` 0))) false false))

(fn `UserConstructionScript`)