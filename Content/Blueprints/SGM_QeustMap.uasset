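; Quest map Blueprint with custom events for restoring saved Narrative quest plugin data.
; LoadTeamSave loads the team's shared Narrative component from its save name, and LoadPlayerData loads "PlayerData" into the first player controller's Narrative component.
; A delayed chain calling both loads and a separate generic Narrative load are left disconnected, so nothing in this Blueprint triggers loading.
; Tick is disabled and the construction script only calls its parent.
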(event `LoadTeamSave`
  (bind _team (`self.Team`))
  (`NarrativeComponent.Load` (`/Game/Blueprints/Narrative/BP_Co-Op.SharedNarrativeComponent` _team) (`/Game/Blueprints/Narrative/BP_Co-Op.Save Name` _team) 0))

(event `LoadPlayerData`
  (bind _asplayer_controller_bp (cast `/Game/Blueprints/PlayerControllerBP` (`GameplayStatics.GetPlayerController` 0))
    (:`then`
      (`NarrativeComponent.Load` (`/Game/Blueprints/PlayerControllerBP.Narrative` _asplayer_controller_bp) "PlayerData" 0))
    (:`CastFailed`
      (`KismetSystemLibrary.PrintString` "PlayerControllerBP Cast FAILED"))))

(fn `UserConstructionScript`
  (`parent.UserConstructionScript`))