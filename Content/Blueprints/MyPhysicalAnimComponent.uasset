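; Actor component that gives a MySCharacter physics-driven hit reactions through a physical animation component it creates at BeginPlay.
; HitReaction applies the "Strong" profile, simulates bodies below the pelvis and adds an impulse along the trace, redirecting pelvis hits to spine_01.
; Each hit extends a decaying timer that Tick uses to set physics blend weight.
; When the timer expires, simulation and ticking switch off.
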(event `self.ReceiveTick`
  (params (DeltaSeconds :type "Float (single-precision)"))
  (bind _output_get (set `self.HitReactionTimeRemaning` (- (`KismetMathLibrary.FClamp` (`KismetMathLibrary.FInterpTo` (`self.HitReactionTimeRemaning`) 0.0 0.0 0.5) 0.0 3.0) (* DeltaSeconds 0.8))))
  (`KismetSystemLibrary.PrintString` (`KismetStringLibrary.Conv_DoubleToString` _output_get))
  (if (<= (`self.HitReactionTimeRemaning`) 0.0)
    (set `self.HitReactionTimeRemaning` 0.0)
    (`SkeletalMeshComponent.SetAllBodiesBelowSimulatePhysics` (`self.Mesh`) "pelvis" false true)
    (`self.SetComponentTickEnabled` false)
    (else
      (`SkeletalMeshComponent.SetAllBodiesBelowPhysicsBlendWeight` (`self.Mesh`) "pelvis" (- (`self.HitReactionTimeRemaning`) 1.0) false true))))

(event `self.ReceiveBeginPlay`
  (bind _returnvalue (`self.GetOwner`))
  (bind _returnvalue_2 (`|AddComponentByClass` _returnvalue "/Script/SavingAndLoading.SPhysicalAnimationComponent"))
  (bind _output_get (set `self.Physical Animation Component` _returnvalue_2))
  (bind _asmy_scharacter (cast `/Game/Blueprints/MySCharacter` _returnvalue))
  (bind _mesh (`Character.Mesh` _asmy_scharacter))
  (`PhysicalAnimationComponent.SetSkeletalMeshComponent` _output_get _mesh)
  (set `self.Mesh` _mesh))

(event `HitReaction`
  (params (Hit :type "HitResult Structure"))
  (bind (_bblockinghit _binitialoverlap _time _distance _location _impactpoint _normal _impactnormal _physmat _hitactor _hitcomponent _hitbonename _hititem _elementindex _faceindex _tracestart _traceend) (`GameplayStatics.BreakHitResult` Hit))
  (`self.SetComponentTickEnabled` true)
  (set `self.HitReactionTimeRemaning` (+ (`self.HitReactionTimeRemaning`) 1.5))
  (`PhysicalAnimationComponent.ApplyPhysicalAnimationProfileBelow` (`self.Physical Animation Component`) "pelvis" "Strong" false false)
  (`SkeletalMeshComponent.SetAllBodiesBelowSimulatePhysics` (`self.Mesh`) "pelvis" true false)
  (`PrimitiveComponent.AddImpulse` (`self.Mesh`) (* (`KismetMathLibrary.Normal` (- _traceend _tracestart)) 5000.0) (select `bool` (== _hitbonename "pelvis") :`false` _hitbonename :`true` "spine_01") true))