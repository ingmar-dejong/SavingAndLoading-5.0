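; BP_StartQuest is an actor that starts a configured Narrative quest when something enters its sphere trigger.
; On overlap, the server begins QuestClass on the overlapping actor's shared Narrative component.
; If the quest starts, it binds to that component's quest-succeeded event and prints a debug string when a quest of that class succeeds.
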(event `self.Sphere.OnComponentBeginOverlap`
  (params (OverlappedComponent :type "PrimitiveComponent Object Reference") (OtherActor :type "Actor Object Reference") (OtherComp :type "PrimitiveComponent Object Reference") (OtherBodyIndex :type Integer) (bFromSweep :type Boolean) (SweepResult :type "HitResult Structure (by ref)"))
  (bind _sharednarrativecomp (`NarrativeComponent.SharedNarrativeComp` (`NarrativeFunctionLibrary.GetNarrativeComponentFromTarget` OtherActor)))
  (`/Engine/EditorBlueprintResources/ActorMacros.Switch Has Authority`
    (:`Authority`
      (bind _returnvalue (`NarrativeComponent.BeginQuest` _sharednarrativecomp (`self.Quest Class`) "None"))
      (`/Engine/EditorBlueprintResources/StandardMacros.IsValid` _returnvalue
        (:`Is Valid`
          (add `NarrativeComponent.OnQuestSucceeded` _sharednarrativecomp (delegate `OnQuestSucceeded_Event_0`)))))))

(event `OnQuestSucceeded_Event_0`
  (params (Quest :type "Quest Object Reference") (QuestSucceededMessage :type "Text (by ref)"))
  (if (== (`GameplayStatics.GetObjectClass` Quest) (`self.Quest Class`))
    (`KismetSystemLibrary.PrintString` "True")))

(fn `UserConstructionScript`)