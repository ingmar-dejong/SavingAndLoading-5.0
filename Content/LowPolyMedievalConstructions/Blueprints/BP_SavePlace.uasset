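; BP_SavePlace is an interactable fire that serves as a world save point.
; Interact flips ActivateFire, calls WriteSaveGame on SGameModeBase, prints a confirmation, then runs UpdateFlames.
; UpdateFlames switches three particle systems and a light to match ActivateFire and records FireActivated, also running on OnActorLoaded.
; OnRep_bFireActivated repeats the visual switch from ActivateFire, while OnRep_bActivateFire is empty.
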(event `Update Flames`
  (bind _lightcomponent0 (`self.LightComponent0`))
  (if (`self.bActivateFire`)
    (`ActorComponent.Activate` (`self.ParticleSystemComponent02`) false)
    (`ActorComponent.Activate` (`self.ParticleSystemComponent01`) false)
    (`ActorComponent.Activate` (`self.ParticleSystemComponent0`) false)
    (`SceneComponent.SetVisibility` _lightcomponent0 true false)
    (set `self.bFireActivated` true)
    (else
      (`ActorComponent.Deactivate` (`self.ParticleSystemComponent0`))
      (`ActorComponent.Deactivate` (`self.ParticleSystemComponent01`))
      (`ActorComponent.Deactivate` (`self.ParticleSystemComponent02`))
      (`SceneComponent.SetVisibility` _lightcomponent0 false false)
      (set `self.bFireActivated` false))))

(event `SGameplayInterface.Interact`
  (params (InstigatorPawn :type "Pawn Object Reference"))
  (if (`self.bFireActivated`)
    (set `self.bActivateFire` false)
    (else
      (set `self.bActivateFire` true)))
  (bind _assgame_mode_base (cast `SGameModeBase` (`GameplayStatics.GetGameMode`)))
  (`SGameModeBase.WriteSaveGame` _assgame_mode_base)
  (`KismetSystemLibrary.PrintString` "WORLD SAVED")
  (`self.Update Flames`))

(event `self.OnActorLoaded`
  (`self.Update Flames`))

(fn `GetInteractText`
  (params (InsitgatorPawn :type "Pawn Object Reference"))
  (returns (ReturnValue :type Text))
  (return ""))

(fn `OnRep_bActivateFire`)

(fn `OnRep_bFireActivated`
  (bind _lightcomponent0 (`self.LightComponent0`))
  (if (`self.bActivateFire`)
    (`ActorComponent.Activate` (`self.ParticleSystemComponent02`) false)
    (`ActorComponent.Activate` (`self.ParticleSystemComponent01`) false)
    (`ActorComponent.Activate` (`self.ParticleSystemComponent0`) false)
    (`SceneComponent.SetVisibility` _lightcomponent0 true false)
    (else
      (`ActorComponent.Deactivate` (`self.ParticleSystemComponent0`))
      (`ActorComponent.Deactivate` (`self.ParticleSystemComponent01`))
      (`ActorComponent.Deactivate` (`self.ParticleSystemComponent02`))
      (`SceneComponent.SetVisibility` _lightcomponent0 false false))))

(fn `UserConstructionScript`)