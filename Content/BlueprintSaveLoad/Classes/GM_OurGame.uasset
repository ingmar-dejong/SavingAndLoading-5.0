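; Game mode that tracks the remaining collectibles and opens the BP_Gate master door when all are collected.
; Registration raises the count; each collection lowers it, updates the player UI, records the ID and triggers an async save.
; BeginPlay waits briefly, refreshes the UI, then loads or creates the SG_Collectible save.
; Loaded data is not applied, collected IDs are never written to the save object, and the change check is an empty stub.
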(event `self.ReceiveBeginPlay`
  (`KismetSystemLibrary.Delay` 0.2)
  (`self.UpdateCollectibleUI`)
  (`self.LoadCollectibles`)
  (`self.CheckForColletableChanges`))

(event `SaveCollectibles`
  (`AsyncActionHandleSaveGame.AsyncSaveGameToSlot` null (`.SlotName` (defaults `/Game/BlueprintSaveLoad/Classes/SG_Collectible` "/Game/BlueprintSaveLoad/Classes/SG_Collectible.SG_Collectible_C"))))

(event `LoadCollectibles`
  (bind (_collecteditems _slotname) (defaults `/Game/BlueprintSaveLoad/Classes/SG_Collectible` "/Game/BlueprintSaveLoad/Classes/SG_Collectible.SG_Collectible_C"))
  (bind _returnvalue (`GameplayStatics.DoesSaveGameExist` _slotname))
  (if _returnvalue
    (`GameplayStatics.LoadGameFromSlot` _slotname)
    (else
      (`GameplayStatics.CreateSaveGameObject` "/Game/BlueprintSaveLoad/Classes/SG_Collectible.SG_Collectible_C"))))

(event `RegisterCollectible`
  (`/Engine/EditorBlueprintResources/StandardMacros.IncrementInt` (`self.NumItemsToCollect`)))

(event `CollectibleCollected`
  (params (ID :type String))
  (`/Engine/EditorBlueprintResources/StandardMacros.DecrementInt` (`self.NumItemsToCollect`)
    (:`  `
      (`self.UpdateCollectibleUI`)
      (`KismetArrayLibrary.Array_AddUnique` (`/Game/BlueprintSaveLoad/Classes/SG_Collectible.CollectedItems`) ID)
      (bind _alldestroyed (`self.CheckForAllCollectiblesDestroyed`))
      (if _alldestroyed
        (`self.OpenMasterDoor`))
      (`self.SaveCollectibles`))))

(fn `CheckForAllCollectiblesDestroyed`
  (returns (AllDestroyed :type Boolean))
  (return (<= (`self.NumItemsToCollect`) 0)))

(fn `CheckForColletableChanges`)

(fn `OpenMasterDoor`
  (bind _returnvalue (`GameplayStatics.GetActorOfClass` "/Game/BlueprintSaveLoad/Blueprints/BP_Gate.BP_Gate_C"))
  (`/Game/BlueprintSaveLoad/Blueprints/BP_Gate.OpenDoor` _returnvalue))

(fn `UpdateCollectibleUI`
  (`/Game/BlueprintSaveLoad/UMG/FINISHED/UMG_PlayerUI_FINISHED.SetCollectibleDisplay` (`self.PlayerUIRef`) (`self.NumItemsToCollect`)))

(fn `UserConstructionScript`)