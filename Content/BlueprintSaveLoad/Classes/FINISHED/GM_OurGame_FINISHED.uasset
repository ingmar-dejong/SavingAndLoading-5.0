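; Game mode for a time-shift level that switches World Partition Data Layers between present and future.
; LoadFuture and LoadPresent read layers from OpenLevel actors, set the layer state, write the game-state slot and call the Game Instance's LoadGame.
; BeginPlay activates the present layer.
; Collectible, foliage, saved-object and layer-save functions are empty stubs, their save and door logic left disconnected, as are the tree loops.
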(event `LoadSaveGame`
  ;[1 1 1] Load our Save Game from storage into a reference then call the change state event on all items that can accept it
)

(event `RegisterCollectible`
  ;[1 1 1] A Collectible wants to register with us
)

(event `CollectibleCollected`
  (params (ID :type String))
  ;[1 1 1] Collectible was Collected, remove it from our number of items to collect then register it in our Save Game object, then see if we have collected them all and open the door if we have, then finally save the game since we did something
)

(event `FoliageCollected`
  (params (`Foliage Transform` :type "Transform Structure") (`Foliage Destroyed` :type Boolean))
  ;[1 1 1] Foliage was collected, add to save file
)

(event `self.ReceiveBeginPlay`
  ;[1 1 1] Begin Play - Load our Save Game
  (`DataLayerSubsystem.SetDataLayerState` (subsystem `DataLayerSubsystem`) (`self.PresentLevelLayer`) "Activated")
  (`KismetSystemLibrary.Delay` 0.2)
  (cast `/Game/BlueprintSaveLoad/Classes/FINISHED/GI_OurGame_FINISHED` (`GameplayStatics.GetGameInstance`)))

(event `LoadFuture`
  (bind _futurelayer (`self.FutureLayer`))
  (bind _in_state (`self.In State`))
  ;[0.512 1 0.1635] Load Future and Save State to SG_GameState
  (bind _output_get (set `self.IsFuture?` true))
  (bind _asgi_our_game_finished (cast `/Game/BlueprintSaveLoad/Classes/FINISHED/GI_OurGame_FINISHED` (`GameplayStatics.GetGameInstance`)))
  (set `self.As GI Our Game FINISHED` _asgi_our_game_finished)
  (bind _returnvalue (`GameplayStatics.GetActorOfClass` "/Game/BlueprintSaveLoad/Blueprints/FINISHED/OpenLevelFuture.OpenLevelFuture_C"))
  (bind _output_get_2 (set `self.Unload Present State` (`/Game/BlueprintSaveLoad/Blueprints/FINISHED/OpenLevelFuture.UnloadPresentState` _returnvalue)))
  (bind _output_get_3 (set `self.PresentLevelLayer` (`/Game/BlueprintSaveLoad/Blueprints/FINISHED/OpenLevelFuture.Present Layer` _returnvalue)))
  (`KismetSystemLibrary.Delay` 0.2)
  (`DataLayerSubsystem.SetDataLayerState` (subsystem `DataLayerSubsystem`) _futurelayer _in_state)
  (bind _output_get_4 (set `self.FutureLayer` _futurelayer))
  (bind _output_get_5 (set `self.In State` _in_state))
  (`self.SaveDataLayerFuture` _output_get_5 _output_get_2 _output_get_4 _output_get_3 (`/Game/BlueprintSaveLoad/Classes/FINISHED/GI_OurGame_FINISHED.GameStateSlot` _asgi_our_game_finished) _output_get)
  (bind _outactors (`GameplayStatics.GetAllActorsOfClass` "/Game/Blueprints/Actors/BP_Present_Tree.BP_Present_Tree_C"))
  (for _ _outactors
    _)
  (`GameplayStatics.SaveGameToSlot` null (`self.GameStateSlot`))
  (`/Game/BlueprintSaveLoad/Classes/FINISHED/GI_OurGame_FINISHED.LoadGame` (`self.As GI Our Game FINISHED`)))

(event `LoadPresent`
  (bind _presentlevellayer (`self.PresentLevelLayer`))
  (bind _presentlayer (`self.PresentLayer`))
  ;[1 0.6788 0.1101] Load Present and Save State to SG_GameState
  (bind _output_get (set `self.IsFuture?` false))
  (bind _asgi_our_game_finished (cast `/Game/BlueprintSaveLoad/Classes/FINISHED/GI_OurGame_FINISHED` (`GameplayStatics.GetGameInstance`)))
  (bind _returnvalue (`GameplayStatics.GetActorOfClass` "/Game/BlueprintSaveLoad/Blueprints/FINISHED/OpenLevelPresent.OpenLevelPresent_C"))
  (bind _output_get_2 (set `self.FutureLayer` (`/Game/BlueprintSaveLoad/Blueprints/FINISHED/OpenLevelPresent.FutureDayler` _returnvalue)))
  (bind _output_get_3 (set `self.Unload State Future` (`/Game/BlueprintSaveLoad/Blueprints/FINISHED/OpenLevelPresent.UnloadStateFuture` _returnvalue)))
  (`DataLayerSubsystem.SetDataLayerState` (subsystem `DataLayerSubsystem`) _presentlevellayer _presentlayer)
  (bind _output_get_4 (set `self.PresentLayer` _presentlayer))
  (bind _output_get_5 (set `self.PresentLevelLayer` _presentlevellayer))
  (`self.SaveDataLayerPresent` (`/Game/BlueprintSaveLoad/Classes/FINISHED/GI_OurGame_FINISHED.GameStateSlot` _asgi_our_game_finished) _output_get_5 _output_get_4 _output_get_3 _output_get_2 _output_get)
  (bind _outactors (`GameplayStatics.GetAllActorsOfClass` "/Game/Blueprints/Actors/FutureTree_BP.FutureTree_BP_C"))
  (for _array_element _outactors
    _)
  (`GameplayStatics.SaveGameToSlot` null (`self.GameStateSlot`))
  (`/Game/BlueprintSaveLoad/Classes/FINISHED/GI_OurGame_FINISHED.LoadGame` (`self.As GI Our Game FINISHED`)))

(fn `ChangeStateFoliage`
  (params (`Input Object` :type "Array of String")))

(fn `ChangeStateOnSavedObjects`)

(fn `CheckForAllCollectiblesDestroyed`
  (returns (AllDestroyed :type Boolean))
  (return (<= (`self.NumItemsToCollect`) 0)))

(fn `CheckForInteractsChanges`)

(fn `OpenMasterDoor`
  ;[1 1 1] Get our door, open it
  (`KismetSystemLibrary.PrintString` "Open Door"))

(fn `SaveDataLayerFuture`
  (params (`Future State` :type "EDataLayerState Enum" :default "Unloaded") (UnloadPresentState :type "EDataLayerState Enum" :default "Unloaded") (`Future Data Layer` :type "ActorDataLayer Structure") (`Present Data Layer` :type "ActorDataLayer Structure") (SlotName :type String) (IsFuture :type Boolean)))

(fn `SaveDataLayerPresent`
  (params (SlotName :type String) (PresentLayer :type "ActorDataLayer Structure") (`Present State` :type "EDataLayerState Enum" :default "Unloaded") (`Future State` :type "EDataLayerState Enum" :default "Unloaded") (FutureLayer :type "ActorDataLayer Structure") (IsFuture :type Boolean)))

(fn `UpdateCollectibleUI`
  (`/Game/BlueprintSaveLoad/UMG/FINISHED/UMG_PlayerUI_FINISHED.SetCollectibleDisplay` (`self.PlayerUIRef`) (`self.NumItemsToCollect`)))

(fn `UserConstructionScript`)