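; Collectible pickup that registers with GM_OurGame_FINISHED on BeginPlay and is destroyed when Custom_Character_FINISHED overlaps its Box or ChangeState fires.
; On destruction it reports its ID to the game mode as collected.
; The construction script assigns a GUID string to any empty ID, giving each pickup a persistent identifier exposed through GetID.
; Interact always returns false.
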(event `self.ReceiveBeginPlay`
  (bind _asgm_our_game_finished (cast `/Game/BlueprintSaveLoad/Classes/FINISHED/GM_OurGame_FINISHED` (`GameplayStatics.GetGameMode`)))
  (`/Game/BlueprintSaveLoad/Classes/FINISHED/GM_OurGame_FINISHED.RegisterCollectible` _asgm_our_game_finished))

(event `/Game/BlueprintSaveLoad/Classes/FINISHED/BPI_SavableState_FINISHED.ChangeState`
  (`KismetSystemLibrary.PrintString` "Change State")
  (`self.K2_DestroyActor`))

(event `self.Box.OnComponentBeginOverlap`
  (params (OverlappedComponent :type "PrimitiveComponent Object Reference") (OtherActor :type "Actor Object Reference") (OtherComp :type "PrimitiveComponent Object Reference") (OtherBodyIndex :type Integer) (bFromSweep :type Boolean) (SweepResult :type "HitResult Structure (by ref)"))
  (cast `/Game/BlueprintSaveLoad/Blueprints/FINISHED/Custom_Character_FINISHED` OtherActor)
  (`self.K2_DestroyActor`))

(event `self.ReceiveDestroyed`
  (bind _asgm_our_game_finished (cast `/Game/BlueprintSaveLoad/Classes/FINISHED/GM_OurGame_FINISHED` (`GameplayStatics.GetGameMode`)))
  (`/Game/BlueprintSaveLoad/Classes/FINISHED/GM_OurGame_FINISHED.CollectibleCollected` _asgm_our_game_finished (`self.ID`)))

(fn `GetID`
  (returns (ID :type String))
  (return (`self.ID`)))

(fn `Interact`
  (returns (`Did Interact?` :type Boolean))
  (return false))

(fn `UserConstructionScript`
  (if (`KismetStringLibrary.IsEmpty` (`self.ID`))
    (set `self.ID` (`KismetGuidLibrary.Conv_GuidToString` (`KismetGuidLibrary.NewGuid`)))))