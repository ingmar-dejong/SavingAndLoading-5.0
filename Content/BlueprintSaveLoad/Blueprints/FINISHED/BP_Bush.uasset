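; BP_Bush is a destructible bush actor for the save/load system, identified by a string ID.
; The construction script fills an empty ID with a new GUID, exposed through GetID.
; ChangeState destroys the actor; Destroyed then passes the ID and BushTransform to GI_OurGame_FINISHED's LoadFoliage with FoliageDestroyed false and debug-prints the transform.
; Interact is empty, and the respawn, collect/plant and level-instance logic is disconnected.
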(event `/Game/BlueprintSaveLoad/Classes/FINISHED/BPI_SavableState_FINISHED.ChangeState`
  (`self.K2_DestroyActor`))

(event `self.ReceiveDestroyed`
  (bind _bush_transform (`self.Bush_Transform`))
  (bind _asgi_our_game_finished (cast `/Game/BlueprintSaveLoad/Classes/FINISHED/GI_OurGame_FINISHED` (`GameplayStatics.GetGameInstance`)))
  (`/Game/BlueprintSaveLoad/Classes/FINISHED/GI_OurGame_FINISHED.LoadFoliage` _asgi_our_game_finished false (`self.ID`) _bush_transform)
  (`KismetSystemLibrary.PrintString` (`KismetStringLibrary.Conv_TransformToString` _bush_transform) true true (struct :`R` 1.0 :`G` 0.339503 :`B` 0.128355 :`A` 1.0) 10.0)
  (cast `/Game/BlueprintSaveLoad/Blueprints/FINISHED/Custom_Character_FINISHED` (`GameplayStatics.GetPlayerCharacter` 0)))

(event `self.ReceiveBeginPlay`)

(fn `GetActorName`
  (returns (Name :type String))
  (return ""))

(fn `GetID`
  (returns (ID :type String))
  (return (`self.ID`)))

(fn `Interact`
  (returns (`Did Interact?` :type Boolean)))

(fn `UserConstructionScript`
  (if (`KismetStringLibrary.EqualEqual_StrStr` (`self.ID`))
    (set `self.ID` (`KismetGuidLibrary.Conv_GuidToString` (`KismetGuidLibrary.NewGuid`)))))